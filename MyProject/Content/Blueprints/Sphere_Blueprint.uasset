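; Sphere actor blueprint that moves from its starting position to an end point and destroys any actor that overlaps it.
; On BeginPlay it caches its location and the world location of Endlocation, then plays a timeline whose OrbMovement track lerps it between them without sweep.
; A separate Hit event only prints "Dead" as on-screen text.
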(event `self.ReceiveHit`
  (params (MyComp :type "PrimitiveComponent Object Reference") (Other :type "Actor Object Reference") (OtherComp :type "PrimitiveComponent Object Reference") (bSelfMoved :type Boolean) (HitLocation :type "Vector Structure") (HitNormal :type "Vector Structure") (NormalImpulse :type "Vector Structure") (Hit :type "HitResult Structure (by ref)"))
  (`KismetSystemLibrary.PrintText` "Dead" true true (struct :`R` 1.0 :`B` 0.192062 :`A` 1.0)))

(event `self.ReceiveActorBeginOverlap`
  (params (OtherActor :type "Actor Object Reference"))
  (`self.K2_DestroyActor` OtherActor))

(event `self.ReceiveBeginPlay`
  (set `self.Endlocatioin` (.location (`SceneComponent.K2_GetComponentToWorld` (`self.Endlocation`))))
  (set `self.StartLocation` (`self.K2_GetActorLocation`))
  (bind (_direction _orbmovement) (`Timeline|MovementTimeline`)
    (:`Update`
      (`self.K2_SetActorLocation` (`KismetMathLibrary.VLerp` (`self.StartLocation`) (`self.Endlocatioin`) _orbmovement)))))

(event `self.ReceiveTick`
  (params (DeltaSeconds :type "Float (single-precision)")))

(fn `UserConstructionScript`)