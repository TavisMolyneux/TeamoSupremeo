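; Ladder actor for a side-scroller that lets the character climb by switching its movement mode.
; Entering the Box trigger sets IsClimbing and puts the SideScrollerCharacter into Flying; leaving clears the flag and restores Walking.
; The flag changes for any overlapping actor, before the character cast.
; While it is set, Tick tries to reapply Flying, but casts the overlapped component rather than the actor to SideScrollerCharacter.
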(event `self.Box.OnComponentBeginOverlap`
  (params (OtherActor :type "Actor Object Reference") (OtherComp :type "PrimitiveComponent Object Reference") (OtherBodyIndex :type Integer) (bFromSweep :type Boolean) (SweepResult :type "HitResult Structure (by ref)"))
  (set `self.IsClimbing` true)
  (bind _asside_scroller_character (cast `/Game/SideScrollerBP/Blueprints/SideScrollerCharacter` OtherActor))
  (`CharacterMovementComponent.SetMovementMode` (`Character.CharacterMovement` _asside_scroller_character) "MOVE_Flying" 0))

(event `self.Box.OnComponentEndOverlap`
  (params (OtherActor :type "Actor Object Reference") (OtherComp :type "PrimitiveComponent Object Reference") (OtherBodyIndex :type Integer))
  (set `self.IsClimbing` false)
  (bind _asside_scroller_character (cast `/Game/SideScrollerBP/Blueprints/SideScrollerCharacter` OtherActor))
  (`CharacterMovementComponent.SetMovementMode` (`Character.CharacterMovement` _asside_scroller_character) "MOVE_Walking" 0))

(event `self.ReceiveTick`
  (params (DeltaSeconds :type "Float (single-precision)"))
  (if (`self.IsClimbing`)
    (bind _asside_scroller_character (cast `/Game/SideScrollerBP/Blueprints/SideScrollerCharacter` (stale `self.Box.OnComponentBeginOverlap` OtherComp)))
    (`CharacterMovementComponent.SetMovementMode` (`Character.CharacterMovement` _asside_scroller_character) "MOVE_Flying" 0)))

(fn `UserConstructionScript`)