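; Checkpoint save system that records progress to a save slot, restores it, and handles slot reset, deletion and level switching.
; SaveCheckPoint writes reached checkpoint values and player data to a CheckPointsave object, using the slot name on Checkpoint actors.
; LoadCheckPoint shares that object with every Checkpoint and, outside multiplayer, moves player 0 to the last checkpoint (linear) or saved location (non-linear).
; Respawn places multiplayer pawns by Checkpoint_Controller PlayerID.
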(fn LoadCheckPoint
  (params (MP :type Boolean :default false))
  (bind _outactors (Actor|GetAllActorsOfClass 0 "/Game/CheckPointBP/Checkpoint.Checkpoint_C"))
  (Utilities|IsValid (Utilities|Array|Get(acopy) _outactors)
    (:Is%20Valid
      (bind _returnvalue (SaveGame|DoesSaveGameExist (Variables|/Game/CheckPointBP/Checkpoint.Checkpoint_C|GetCheckPoint%20Slot%20Name (Utilities|Array|Get(acopy) _outactors))))
      (if _returnvalue
        (bind _returnvalue_2 (SaveGame|LoadGamefromSlot (Variables|/Game/CheckPointBP/Checkpoint.Checkpoint_C|GetCheckPoint%20Slot%20Name (Utilities|Array|Get(acopy) _outactors))))
        (bind _ascheck_pointsave (Utilities|Casting|CastToCheckPointsave _returnvalue_2))
        (bind _output_get (LocalVariables|SetSave%20Ref _ascheck_pointsave))
        (LocalVariables|SetPlayerRot (Variables|/Game/CheckPointBP/Blueprint/CheckPointsave.CheckPointsave_C|GetPlayerRotation _output_get))
        (bind _outactors_2 (Actor|GetAllActorsOfClass 0 "/Game/CheckPointBP/Checkpoint.Checkpoint_C"))
        (for (_array_element _array_index) (Variables|/Game/CheckPointBP/Blueprint/CheckPointsave.CheckPointsave_C|GetCheckPointValue _ascheck_pointsave) ; Find the Highest Check Point Value
          (if (> _array_element (Utilities|Array|Get(acopy) (Variables|/Game/CheckPointBP/Blueprint/CheckPointsave.CheckPointsave_C|GetCheckPointValue _ascheck_pointsave) (- _array_index 1)))
            (bind _output_get_2 (Variables|/Game/CheckPointBP/Blueprint/CheckPointsave.CheckPointsave_C|SetLastCheckPointValue _ascheck_pointsave _array_element))))
        (for _array_element_2 _outactors_2
          (Variables|/Game/CheckPointBP/Checkpoint.Checkpoint_C|SetSaveGameRef _array_element_2 _ascheck_pointsave)
          (if (and (!= (Utilities|Array|FindItem (Variables|/Game/CheckPointBP/Blueprint/CheckPointsave.CheckPointsave_C|GetCheckPointValue _ascheck_pointsave) (Variables|/Game/CheckPointBP/Checkpoint.Checkpoint_C|GetCheckPointValue _array_element_2)) -1) (not MP))
            (Default|ForMultiplayer _array_element_2)
            (if (== (Variables|/Game/CheckPointBP/Checkpoint.Checkpoint_C|GetCheckPointValue _array_element_2) _output_get_2)
              (if (Variables|/Game/CheckPointBP/Blueprint/CheckPointsave.CheckPointsave_C|GetLinearOr (LocalVariables|GetSave%20Ref))
                ;[0.286 1 0.1792] Linear
                (bind _outactors_3 (Actor|GetAllActorsOfClass 0 "/Game/CheckPointBP/Checkpoint.Checkpoint_C"))
                (for (_array_element_3 _array_index_2) _outactors_3
                  (if (== (Variables|/Game/CheckPointBP/Checkpoint.Checkpoint_C|GetCheckPointValue _array_element_3) _output_get_2)
                    (LocalVariables|SetPlayerRot (Variables|/Game/CheckPointBP/Checkpoint.Checkpoint_C|GetPlayer%20Rotation _array_element_3))))
                (Transformation|SetWorldTransform (Game|GetPlayerCharacter 0) (Math|Transform|MakeTransform (Math|Vector|MakeVector (+ (.X (Math|Vector|BreakVector (Transformation|GetWorldLocation _array_element_2))) (Variables|/Game/CheckPointBP/Checkpoint.Checkpoint_C|GetXOffsetToSpawnTo _array_element_2)) (+ (.Y (Math|Vector|BreakVector (Transformation|GetWorldLocation _array_element_2))) (Variables|/Game/CheckPointBP/Checkpoint.Checkpoint_C|GetYOffsetToSpawnTo _array_element_2)) (+ (.Z (Math|Vector|BreakVector (Transformation|GetWorldLocation _array_element_2))) (Variables|/Game/CheckPointBP/Checkpoint.Checkpoint_C|GetZOffsetToSpawnTo _array_element_2))) (LocalVariables|GetPlayerRot)) false)
                (Pawn|SetControlRotation (Game|GetPlayerController 0) (LocalVariables|GetPlayerRot))
                (else
                  ;[0.9778 1 0.2394] None-Linear
                  (Transformation|SetWorldTransform (Game|GetPlayerCharacter 0) (Math|Transform|MakeTransform (Math|Vector|MakeVector (+ (.X (Math|Vector|BreakVector (Utilities|Array|Get(acopy) (Variables|/Game/CheckPointBP/Blueprint/CheckPointsave.CheckPointsave_C|GetPlayerLocation (LocalVariables|GetSave%20Ref))))) (Variables|/Game/CheckPointBP/Checkpoint.Checkpoint_C|GetXOffsetToSpawnTo _array_element_2)) (+ (.Y (Math|Vector|BreakVector (Utilities|Array|Get(acopy) (Variables|/Game/CheckPointBP/Blueprint/CheckPointsave.CheckPointsave_C|GetPlayerLocation (LocalVariables|GetSave%20Ref))))) (Variables|/Game/CheckPointBP/Checkpoint.Checkpoint_C|GetYOffsetToSpawnTo _array_element_2)) (+ (.Z (Math|Vector|BreakVector (Utilities|Array|Get(acopy) (Variables|/Game/CheckPointBP/Blueprint/CheckPointsave.CheckPointsave_C|GetPlayerLocation (LocalVariables|GetSave%20Ref))))) (Variables|/Game/CheckPointBP/Checkpoint.Checkpoint_C|GetZOffsetToSpawnTo _array_element_2))) (LocalVariables|GetPlayerRot)) false)
                  (Pawn|SetControlRotation (Game|GetPlayerController 0) (LocalVariables|GetPlayerRot)))))))
        (else
          ;[1 0.5026 0.9986] CreateSave Object
          (bind _returnvalue_3 (SaveGame|CreateSaveGameObject "/Game/CheckPointBP/Blueprint/CheckPointsave.CheckPointsave_C")) ; Choose Save Game Class Here
          (bind _ascheck_pointsave_2 (Utilities|Casting|CastToCheckPointsave _returnvalue_3))
          (bind _outactors_4 (Actor|GetAllActorsOfClass 0 "/Game/CheckPointBP/Checkpoint.Checkpoint_C"))
          (for _array_element_4 _outactors_4
            (Variables|/Game/CheckPointBP/Checkpoint.Checkpoint_C|SetSaveGameRef _array_element_4 _ascheck_pointsave_2)))))))

(fn SaveCheckPoint
  (params (ActorLocation :type Array%20of%20Vectors) (CheckPointValue :type Integer :default 0) (CheckPointslotName :type String) (CheckPoint%20Save%20Red :type Check%20Pointsave%20Object%20Reference) (Linear :type Boolean :default false) (PlayerRot :type Rotator :default "0, 0, 0") (PlayerVar :type Array%20of%20Floats%20%28single-precision%29))
  (bind _output_get (LocalVariables|SetSaveGameRef CheckPoint%20Save%20Red))
  (Variables|/Game/CheckPointBP/Blueprint/CheckPointsave.CheckPointsave_C|SetLinearOr _output_get Linear)
  (Variables|/Game/CheckPointBP/Blueprint/CheckPointsave.CheckPointsave_C|SetPlayerRotation _output_get PlayerRot)
  (Variables|/Game/CheckPointBP/Blueprint/CheckPointsave.CheckPointsave_C|SetPlayerVariables _output_get PlayerVar)
  (Variables|/Game/CheckPointBP/Blueprint/CheckPointsave.CheckPointsave_C|SetPlayerLocation _output_get ActorLocation)
  (Variables|/Game/CheckPointBP/Blueprint/CheckPointsave.CheckPointsave_C|SetLastCheckPointValue (LocalVariables|GetSaveGameRef) CheckPointValue)
  (Utilities|Array|AddUnique (Variables|/Game/CheckPointBP/Blueprint/CheckPointsave.CheckPointsave_C|GetCheckPointValue (LocalVariables|GetSaveGameRef)) CheckPointValue)
  (SaveGame|SaveGametoSlot (LocalVariables|GetSaveGameRef) CheckPointslotName))

(fn DeleteSaveslot
  (bind _outactors (Actor|GetAllActorsOfClass 0 "/Game/CheckPointBP/Checkpoint.Checkpoint_C"))
  (Utilities|IsValid (Utilities|Array|Get(acopy) _outactors)
    (:Is%20Valid
      (bind _returnvalue (SaveGame|DoesSaveGameExist (Variables|/Game/CheckPointBP/Checkpoint.Checkpoint_C|GetCheckPoint%20Slot%20Name (Utilities|Array|Get(acopy) _outactors))))
      (if _returnvalue
        (SaveGame|DeleteGameinSlot (Variables|/Game/CheckPointBP/Checkpoint.Checkpoint_C|GetCheckPoint%20Slot%20Name (Utilities|Array|Get(acopy) _outactors)))))))

(fn LoadLevel
  (params (Level :type Levels%20Enum :default "NewEnumerator0"))
  (CallFunction|ResetSlot)
  (switch Utilities|FlowControl|Switch|SwitchonLevels Level
    (:NewEnumerator0
      (Game|OpenLevel(byName) 0 "Level1" false))
    (:NewEnumerator1
      (Game|OpenLevel(byName) 0 "Level2" false))))

(fn ResetSlot
  (bind _outactors (Actor|GetAllActorsOfClass 0 "/Game/CheckPointBP/Checkpoint.Checkpoint_C"))
  (Utilities|IsValid (Utilities|Array|Get(acopy) _outactors)
    (:Is%20Valid
      (bind _returnvalue (SaveGame|DoesSaveGameExist (Variables|/Game/CheckPointBP/Checkpoint.Checkpoint_C|GetCheckPoint%20Slot%20Name (Utilities|Array|Get(acopy) _outactors))))
      (if _returnvalue
        (Variables|/Game/CheckPointBP/Blueprint/CheckPointsave.CheckPointsave_C|SetPlayerLocation (Variables|/Game/CheckPointBP/Checkpoint.Checkpoint_C|GetSaveGameRef (Utilities|Array|Get(acopy) _outactors)) (Utilities|Array|MakeArray "0, 0, 0"))
        (Utilities|Array|Clear (Variables|/Game/CheckPointBP/Blueprint/CheckPointsave.CheckPointsave_C|GetCheckPointValue (Variables|/Game/CheckPointBP/Checkpoint.Checkpoint_C|GetSaveGameRef (Utilities|Array|Get(acopy) _outactors))))
        (Variables|/Game/CheckPointBP/Blueprint/CheckPointsave.CheckPointsave_C|SetLastCheckPointValue (Variables|/Game/CheckPointBP/Checkpoint.Checkpoint_C|GetSaveGameRef (Utilities|Array|Get(acopy) _outactors)) -1)
        (Utilities|Array|Clear (Variables|/Game/CheckPointBP/Blueprint/CheckPointsave.CheckPointsave_C|GetPlayerVariables (Variables|/Game/CheckPointBP/Checkpoint.Checkpoint_C|GetSaveGameRef (Utilities|Array|Get(acopy) _outactors))))
        (SaveGame|SaveGametoSlot (Variables|/Game/CheckPointBP/Checkpoint.Checkpoint_C|GetSaveGameRef (Utilities|Array|Get(acopy) _outactors)) (Variables|/Game/CheckPointBP/Checkpoint.Checkpoint_C|GetCheckPoint%20Slot%20Name (Utilities|Array|Get(acopy) _outactors)))))))

(fn Respawn
  (params (ID :type Integer :default 0))
  ;[1 1 1] Multiplayer Respawn
  (bind _outactors (Actor|GetAllActorsOfClass 0 "/Game/CheckPointBP/Checkpoint.Checkpoint_C"))
  (bind _outactors_2 (Actor|GetAllActorsOfClass 0 "/Game/CheckPointBP/Blueprint/Checkpoint_Controller.Checkpoint_Controller_C"))
  (for _array_element _outactors_2
    (if (== (Variables|/Game/CheckPointBP/Blueprint/Checkpoint_Controller.Checkpoint_Controller_C|GetPlayer%20ID _array_element) ID)
      (Transformation|SetActorTransform (Pawn|GetControlledPawn _array_element) (Math|Transform|MakeTransform (Utilities|Array|Get(acopy) (Variables|/Game/CheckPointBP/Blueprint/CheckPointsave.CheckPointsave_C|GetPlayerLocation (Variables|/Game/CheckPointBP/Checkpoint.Checkpoint_C|GetSaveGameRef (Utilities|Array|Get(acopy) _outactors))) ID) (Variables|/Game/CheckPointBP/Blueprint/CheckPointsave.CheckPointsave_C|GetPlayerRotation (Variables|/Game/CheckPointBP/Checkpoint.Checkpoint_C|GetSaveGameRef (Utilities|Array|Get(acopy) _outactors)))))
      (Pawn|SetControlRotation (Game|GetPlayerController 0) (Variables|/Game/CheckPointBP/Blueprint/CheckPointsave.CheckPointsave_C|GetPlayerRotation (Variables|/Game/CheckPointBP/Checkpoint.Checkpoint_C|GetSaveGameRef (Utilities|Array|Get(acopy) _outactors))))
      (Development|PrintString 0))))