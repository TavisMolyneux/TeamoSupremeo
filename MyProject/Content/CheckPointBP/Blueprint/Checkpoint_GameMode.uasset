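; Game mode for a checkpoint system that tracks and saves player locations for multiplayer.
; On login, it gives each Checkpoint_Controller an incrementing ID, tags its pawn "hero" and stores the spawn location by ID.
; After a short retriggerable delay, it saves all locations using the first Checkpoint actor's settings, if that checkpoint is multiplayer.
; SaveLocation updates one player's entry and saves the whole array again.
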(event `self.K2_PostLogin`
  (params (NewPlayer :type "PlayerController Object Reference"))
  ;[1 1 1] Set Player Id and Initial Location
  (bind _ascheckpoint_controller (cast `/Game/CheckPointBP/Blueprint/Checkpoint_Controller` NewPlayer))
  (bind _output_get (set `/Game/CheckPointBP/Blueprint/Checkpoint_Controller.Player ID` (`self.Next Payer ID`) _ascheckpoint_controller))
  (set `self.Next Payer ID` (+ (`self.Next Payer ID`) 1))
  (`KismetArrayLibrary.Array_AddUnique` (`self.Player Index`) _ascheckpoint_controller)
  (bind _returnvalue (`Controller.K2_GetPawn` _ascheckpoint_controller))
  (set `Actor.Tags` (`|MakeArray` "hero" :!type "Name") _returnvalue)
  (`KismetArrayLibrary.Array_Set` (`self.PlayerLocations`) _output_get (`self.K2_GetActorLocation` _returnvalue) true)
  (`KismetSystemLibrary.RetriggerableDelay` 0.1)
  (bind _outactors (`GameplayStatics.GetAllActorsOfClass` "/Game/CheckPointBP/Checkpoint.Checkpoint_C"))
  (bind _item (`KismetArrayLibrary.Array_Get` _outactors))
  (if (`/Game/CheckPointBP/Checkpoint.Multiplayer` _item)
    (`/Game/CheckPointBP/Blueprint/SaveLoadCheckPoint.SaveCheckPoint` (`self.PlayerLocations`) (`/Game/CheckPointBP/Checkpoint.CheckPointValue` _item) (`/Game/CheckPointBP/Checkpoint.CheckPoint Slot Name` _item) (`/Game/CheckPointBP/Checkpoint.SaveGameRef` _item) (`/Game/CheckPointBP/Checkpoint.Linear` _item) (`/Game/CheckPointBP/Checkpoint.Player Rotation` _item) (`|MakeArray` 0.0 :!type "Float (single-precision)"))))

(event `Save Location`
  (params (Location :type "Object.Vector Structure" :default (0.0 0.0 0.0)) (ID :type Integer :default 0) (Value :type Integer :default 0) (`Slot Name` :type String) (`save ref` :type "/Game/CheckPointBP/Blueprint/CheckPointsave Object Reference") (linearor :type Boolean :default false) (`player rotation` :type "Object.Rotator Structure" :default (struct)))
  ;[1 1 1] Save Multiplayer Location
  (`KismetArrayLibrary.Array_Set` (`self.PlayerLocations`) ID Location true)
  (`/Game/CheckPointBP/Blueprint/SaveLoadCheckPoint.SaveCheckPoint` (`self.PlayerLocations`) Value `Slot Name` `save ref` linearor `player rotation` (`|MakeArray` 0.0 :!type "Float (single-precision)")))

(fn `UserConstructionScript`)